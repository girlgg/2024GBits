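; BP_Item_Drawer is a Level01 drawer item that slides once the player has the required item.
; PlayerHasItem starts the slide and turns off further interaction.
; Tick then moves the actor along world -Y in fixed per-frame steps until AddDis reaches AllDis, so speed depends on frame rate and direction ignores the drawer's rotation.
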(event `self.ReceiveTick`
  (params (DeltaSeconds :type "Float (single-precision)"))
  (`parent.ReceiveTick` DeltaSeconds)
  (if (and (`self.PlayAnim`) (> (`self.AllDis`) (`self.AddDis`)))
    (`self.K2_AddActorWorldTransform` (`KismetMathLibrary.MakeTransform` (0.0 -2.0 0.0)))
    (set `self.AddDis` (+ (`self.AddDis`) 2.0))))

(event `self.PlayerHasItem`
  (set `self.PlayAnim` true)
  (set `self.bAllowInteract` false))

(fn `UserConstructionScript`
  (`parent.UserConstructionScript`))