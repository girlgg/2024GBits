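; BP_Item_Oven is an interactive Level01 puzzle item that takes a plate and an egg, then leads to the next level.
; It unlocks interaction on the second IntoDream event.
; PlayerHasItem advances flag-tracked stages by rewriting the required inventory item name: Egg after the plate, then empty after the egg.
; Any later PlayerHasItem call spawns BP_Item_NextLevel at a hardcoded location.
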(event `self.K2_IntoDream`
  (`/Engine/EditorBlueprintResources/StandardMacros.IncrementInt` (`self.DreamTimes`)
    (:`  `
      (if (== (`self.DreamTimes`) 2)
        (set `self.bAllowInteract` true)))))

(event `self.PlayerHasItem`
  (if (`self.bGetPlate`)
    (if (`self.bGetEgg`)
      (`|SpawnActorFromClass` "/Game/Levels/Level01/Items/BP_Item_NextLevel.BP_Item_NextLevel_C" (`KismetMathLibrary.MakeTransform` (760.0 890.0 144.0)) "Undefined" "MultiplyWithRoot" null null)
      (else
        (`|VariableSetRef` (`.InventoryItemName` (break `InteractionMethods` (`.InteractionMethod` (break `InteractiveData` (`self.InteractiveData`))))))
        (set `self.bGetEgg` true)))
    (else
      (`|VariableSetRef` (`.InventoryItemName` (break `InteractionMethods` (`.InteractionMethod` (break `InteractiveData` (`self.InteractiveData`))))) "Egg")
      (set `self.bGetPlate` true))))

(fn `UserConstructionScript`
  (`parent.UserConstructionScript`))