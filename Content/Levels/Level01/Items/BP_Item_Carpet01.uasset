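; Carpet item for Level01 that becomes interactable the second time the IntoDream event fires.
; Its PlayerHasItem event rotates the mesh in 90-degree steps, counting each turn.
; Once it has turned twice, the next call disables interaction and adds Carpet01 to the player inventory as a pickup hidden from the inventory display.
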(event `self.K2_IntoDream`
  (`/Engine/EditorBlueprintResources/StandardMacros.IncrementInt` (`self.IntoDreamTimes`)
    (:`  `
      (if (== (`self.IntoDreamTimes`) 2)
        (set `self.bAllowInteract` true)))))

(event `self.PlayerHasItem`
  (if (== (`self.RotatorTimes`) 2)
    (set `self.bAllowInteract` false)
    (`GameplayFunctinos.AddItemToPlayerInventory` self (make `InteractiveData` "Carpet01" null 0.0 (0.0 0.0 0.0) (make `InteractionMethods` "Pickup" "" "/Engine/ArtTools/RenderToTexture/Textures/127grey.127grey" false)))
    (else
      (`SceneComponent.K2_AddRelativeRotation` (`self.Mesh`) (struct :`Yaw` 90.0) false false)
      (`/Engine/EditorBlueprintResources/StandardMacros.IncrementInt` (`self.RotatorTimes`)))))

(fn `UserConstructionScript`
  (`parent.UserConstructionScript`))