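; BP_Item_Vase01 is a Level01 vase item that plays protagonist dialogue when the PlayerHasItem event fires.
; The event hides the mesh, then caches the game mode as LevelGameModeBase and calls its ShowTitle with InPause enabled.
; The two timed subtitles say it is still early to sleep more, but the sleeping pills are gone, so another way to fall asleep is needed.
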(event `self.PlayerHasItem`
  (`|ExecutionSequence`
    (:`then_0`
      (`SceneComponent.SetVisibility` (`self.Mesh`) false false))
    (:`then_1`
      (bind _aslevel_game_mode_base (cast `LevelGameModeBase` (`GameplayStatics.GetGameMode`)))
      (set `self.As Level Game Mode Base` _aslevel_game_mode_base))
    (:`then_2`
      (`LevelGameModeBase.ShowTitle` (`self.As Level Game Mode Base`) "" (`|MakeArray` (make `SubtitleSetting` "主角：看来时间还早，我还得再睡会儿") (make `SubtitleSetting` "主角：安眠药已经吃完了，看来想睡着还得再找个办法")) true))))

(fn `UserConstructionScript`
  (`parent.UserConstructionScript`))