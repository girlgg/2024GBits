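; Level01 pendulum item that the player interacts with in two stages, serving as a gaze-triggered way into a dream.
; PlayerHasItem advances a counter: the first call allows interaction, switches the interaction method to IntoDream and turns on timed gaze interaction.
; The second call hides the mesh and has LevelGameModeBase show a delayed protagonist subtitle hinting at what to do next.
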(event `self.PlayerHasItem`
  (`/Engine/EditorBlueprintResources/StandardMacros.IncrementInt` (`self.InterNum`)
    (:`  `
      (switch `int` (`self.InterNum`)
        (:`1`
          (set `self.bAllowInteract` true)
          (`|VariableSetRef` (break `InteractionMethods` (`.InteractionMethod` (break `InteractiveData` (`self.InteractiveData`)))) "IntoDream")
          (set `self.bIsGazeInteraction` true)
          (set `self.GazeDuration` 5.0))
        (:`2`
          (`SceneComponent.SetVisibility` (`self.Mesh`) false false)
          (bind _aslevel_game_mode_base (cast `LevelGameModeBase` (`GameplayStatics.GetGameMode`)))
          (`LevelGameModeBase.ShowTitle` _aslevel_game_mode_base "" (`|MakeArray` (make `SubtitleSetting` "主角：……你应该知道怎么做了吧")) false))))))

(fn `UserConstructionScript`
  (`parent.UserConstructionScript`))