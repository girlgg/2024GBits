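; Level 01 hypnotic item pickup that plays a story beat when the player obtains it.
; On PlayerHasItem, it hides its mesh and shows three timed protagonist subtitles about sleep paralysis and needing noise to wake up, via LevelGameModeBase's ShowTitle without pausing.
; It also spawns a Block at a hardcoded world position and passes five seconds to its DestroyTime.
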(event `self.PlayerHasItem`
  (`|ExecutionSequence`
    (:`then_0`
      (`SceneComponent.SetVisibility` (`self.Mesh`) false false))
    (:`then_1`
      (bind _aslevel_game_mode_base (cast `LevelGameModeBase` (`GameplayStatics.GetGameMode`)))
      (`LevelGameModeBase.ShowTitle` _aslevel_game_mode_base "" (`|MakeArray` (make `SubtitleSetting` "主角：我就知道，又来了……") (make `SubtitleSetting` "主角：失眠症和睡眠瘫痪症为什么会同时发生在我身上……") (make `SubtitleSetting` "主角：快没时间了，我得找个办法醒来，比如……制造点大动静……")) false))
    (:`then_2`
      (bind _returnvalue (`|SpawnActorFromClass` "/Game/Levels/Intro/Items/Block.Block_C" (`KismetMathLibrary.MakeTransform` (1300.0 1200.0 500.0)) "Undefined" "MultiplyWithRoot" null null))
      (`/Game/Levels/Intro/Items/Block.DestroyTime` _returnvalue 5.0))))

(fn `UserConstructionScript`
  (`parent.UserConstructionScript`))