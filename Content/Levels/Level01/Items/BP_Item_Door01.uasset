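; BP_Item_Door01 is a Level01 interactive door that reacts to the player having an item and to dream-state changes.
; PlayerHasItem hides the mesh, disables its collision, sets AllowIn and switches the interaction method to Door.
; Once AllowIn is set, IntoDream shows the mesh and OutDream hides it, with both setting AllowInteract to true.
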(event `self.PlayerHasItem`
  (bind _mesh (`self.Mesh`))
  (`SceneComponent.SetVisibility` _mesh false false)
  (`PrimitiveComponent.SetCollisionEnabled` _mesh "NoCollision")
  (set `self.bAllowIn` true)
  (`|VariableSetRef` (break `InteractionMethods` (`.InteractionMethod` (break `InteractiveData` (`self.InteractiveData`)))) "Door"))

(event `self.K2_IntoDream`
  (if (`self.bAllowIn`)
    (`SceneComponent.SetVisibility` (`self.Mesh`) true false)
    (set `self.bAllowInteract` true)))

(event `self.K2_OutDream`
  (if (`self.bAllowIn`)
    (`SceneComponent.SetVisibility` (`self.Mesh`) false false)
    (set `self.bAllowInteract` true)))

(fn `UserConstructionScript`
  (`parent.UserConstructionScript`))