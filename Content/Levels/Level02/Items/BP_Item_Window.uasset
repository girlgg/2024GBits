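; BP_Item_Window is a Level02 interactable window item that puts the player to sleep.
; Both interaction options share one path: show a subtitle saying a ball knocked the player out, then call IntoDream on the player's InteractionManager.
; The item then disables interaction and response and destroys itself.
; Its PlayerHasItem, IntoDream and OutDream events are empty.
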(event `self.PlayerHasItem`)

(event `self.K2_IntoDream`)

(event `self.K2_OutDream`)

(event `self.K2_Option1`
  (bind _aslevel_game_mode_base (cast `LevelGameModeBase` (`GameplayStatics.GetGameMode`) :!label _label))
  (`LevelGameModeBase.ShowTitle` _aslevel_game_mode_base "" (`|MakeArray` (make `SubtitleSetting` "你被球击中了，直接陷入了沉睡" 2.0)) false)
  (bind _returnvalue (`GameplayFunctinos.GetPlayer` self))
  (`InteractionManagerComponent.IntoDream` (`FirstPersonPlayerBase.InteractionManager` _returnvalue) 5.0)
  (set `self.bAllowInteract` false)
  (set `self.bAllowResponse` false)
  (`self.K2_DestroyActor`))

(event `self.K2_Option2`
  (goto _label))

(fn `UserConstructionScript`
  (`parent.UserConstructionScript`))