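; BP_Item_CollectionCabinet01 is an interactable collection cabinet in Level02 that is visible and interactable only outside the dream state.
; It records two successive option picks in FirstOp and SecondOp.
; After the second pick, choosing option 2 first, or option 1 then 2, calls IntoDream on the player's InteractionManager with differing values.
; Every completed sequence then ends the reply input and destroys the cabinet.
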(event `self.K2_OutDream`
  (`SceneComponent.SetVisibility` (`self.Mesh`) true false)
  (set `self.bAllowInteract` true))

(event `self.K2_IntoDream`
  (`SceneComponent.SetVisibility` (`self.Mesh`) false false)
  (set `self.bAllowInteract` false))

(event `self.K2_Option1`
  (if (== (`self.FirstOp`) 0)
    (set `self.FirstOp` 1)
    (elif (== (`self.SecondOp`) 0)
      (set `self.SecondOp` 1)
      (`|ExecutionSequence` :!label _label
        (:`then_0`
          (switch `int` (`self.FirstOp`)
            (:`1`
              (switch `int` (`self.SecondOp`)
                (:`2`
                  (bind _returnvalue (`GameplayFunctinos.GetPlayer` self))
                  (`InteractionManagerComponent.IntoDream` (`FirstPersonPlayerBase.InteractionManager` _returnvalue) 2.0))))
            (:`2`
              (bind _returnvalue_2 (`GameplayFunctinos.GetPlayer` self))
              (`InteractionManagerComponent.IntoDream` (`FirstPersonPlayerBase.InteractionManager` _returnvalue_2) 5.0))))
        (:`then_1`
          (`self.InputEndRelies`)
          (`self.K2_DestroyActor`))))))

(event `self.K2_Option2`
  (if (== (`self.FirstOp`) 0)
    (set `self.FirstOp` 2)
    (elif (== (`self.SecondOp`) 0)
      (set `self.SecondOp` 2)
      (goto _label))))

(fn `UserConstructionScript`)