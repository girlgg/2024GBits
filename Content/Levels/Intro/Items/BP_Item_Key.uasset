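; BP_Item_Key is the intro level's key item, which triggers a short story beat when the player has it.
; Its PlayerHasItem event spawns a temporary Block at a fixed location and plays protagonist subtitles through LevelGameModeBase about sleep paralysis and waking up by making noise.
; The Block is destroyed after a short fixed delay, independent of any subtitle completion callback.
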(event `self.PlayerHasItem`
  (bind _aslevel_game_mode_base (cast `LevelGameModeBase` (`GameplayStatics.GetGameMode`)))
  (bind _returnvalue (`|SpawnActorFromClass` "/Game/Levels/Intro/Items/Block.Block_C" (`KismetMathLibrary.MakeTransform` (0.0 0.0 500.0)) "Undefined" "MultiplyWithRoot" null null))
  (`LevelGameModeBase.PlaySubtitles` _aslevel_game_mode_base (`|MakeArray` (make `SubtitleSetting` "主角：我就知道，又来了……") (make `SubtitleSetting` "主角：失眠症和睡眠瘫痪症为什么会同时发生在我身上……") (make `SubtitleSetting` "主角：快没时间了，我得找个办法醒来，比如……制造点大动静……")))
  (`KismetSystemLibrary.Delay` 3.0)
  (`self.K2_DestroyActor` _returnvalue))

(fn `UserConstructionScript`
  (`parent.UserConstructionScript`))